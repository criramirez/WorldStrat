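; Main building actor for a civilization that periodically spawns NPC units and grows that civilization's population.
; On BeginPlay it finds the civilization object matching its Civilizacion in the GameInstanceCR list and starts a looping GenerarUnidades timer.
; Each tick of that timer spawns a BP_NPCBase offset from the building, tags and labels it with the civilization, and increments Poblacion without checking LimitePoblacion.
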(event EventBeginPlay
  (bind _asgame_instance_cr (Utilities|Casting|CastToGameInstanceCR (Game|GetGameInstance)))
  (bind _civilizaciones_cargadas (Default|SetBpCivilizaciones _asgame_instance_cr))
  (for _array_element _civilizaciones_cargadas
    (if (Utilities|Enum|Equal(Enum) (.civilizacion (Variables|/Game/Blueprints/Mundo/BP_Civilizacion.BP_Civilizacion_C|GetEST_Civi _array_element)) (Variables|Default|Getcivilizacion))
      (Variables|Default|SetBP_Civ _array_element)
      (Utilities|Time|SetTimerbyFunctionName 0 "GenerarUnidades" (Variables|Default|GettiempoEsperaUnidad) true))))

(event Collision|EventActorBeginOverlap
  (params (OtherActor :type Actor%20Object%20Reference)))

(event EventTick
  (params (DeltaSeconds :type Float%20%28single-precision%29)))

(fn ConstructionScript)

(fn GenerarUnidades
  (bind _returnvalue (Transformation|GetActorLocation))
  (bind _bp_civ (Variables|Default|GetBP_Civ))
  (bind _civilizacion (Variables|Default|Getcivilizacion))
  (bind _returnvalue_2 (Game|SpawnActorfromClass "/Game/Blueprints/Mundo/NPC/BP_NPCBase.BP_NPCBase_C" (Math|Transform|MakeTransform (Math|Vector|MakeVector (- (.x _returnvalue) 5e+02) (.y _returnvalue) (.z _returnvalue)) "0,180.000000, 0" "1,1,1") "AdjustIfPossibleButDontSpawnIfColliding" 0 "NewEnumerator1" false 0))
  (Utilities|IsValid _returnvalue_2
    (:Is%20Valid
      (Variables|Default|SetNPC_BaseAux _returnvalue_2)
      (Variables|/Game/Blueprints/Mundo/NPC/BP_NPCBase.BP_NPCBase_C|SetEST_Npc (Variables|Default|GetNPC_BaseAux) (Utilities|Struct|MakeEST_NPC (.id (Variables|/Game/Blueprints/Mundo/NPC/BP_NPCBase.BP_NPCBase_C|GetEST_Npc (Variables|Default|GetNPC_BaseAux))) (.vida (Variables|/Game/Blueprints/Mundo/NPC/BP_NPCBase.BP_NPCBase_C|GetEST_Npc (Variables|Default|GetNPC_BaseAux))) _civilizacion))
      (Rendering|Components|TextRender|SetText (Variables|/Game/Blueprints/Mundo/NPC/BP_NPCBase.BP_NPCBase_C|GetTextRender (Variables|Default|GetNPC_BaseAux)) (Utilities|Text|ToText(String) (Utilities|String|EnumtoString _civilizacion)))
      (bind _result (Math|Integer|IncrementInt (.poblacion (Variables|/Game/Blueprints/Mundo/BP_Civilizacion.BP_Civilizacion_C|GetEST_Civi _bp_civ)))
        (:%20%20
          (Variables|/Game/Blueprints/Mundo/BP_Civilizacion.BP_Civilizacion_C|SetEST_Civi _bp_civ (Utilities|Struct|MakeEST_Civilizacion (.civilizacion (Variables|/Game/Blueprints/Mundo/BP_Civilizacion.BP_Civilizacion_C|GetEST_Civi _bp_civ)) _result (.limitepoblacion (Variables|/Game/Blueprints/Mundo/BP_Civilizacion.BP_Civilizacion_C|GetEST_Civi _bp_civ)) (.comida (Variables|/Game/Blueprints/Mundo/BP_Civilizacion.BP_Civilizacion_C|GetEST_Civi _bp_civ)))))))))