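; BP_EdificioPrincipal is a civilization's main building, which periodically produces NPC units for it.
; InicializarCiv looks up the civilization through GameInstanceCR, raises its population capacity and starts a looping timer on GenerarUnidades.
; While capacity remains, GenerarUnidades spawns a BP_NPCBase offset from the building, assigns its civilization and registers it in the population count and NPC list.
; BeginPlay is empty, and older direct struct-editing code remains disconnected.
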(event EventBeginPlay)

(event Collision|EventActorBeginOverlap
  (params (OtherActor :type Actor%20Object%20Reference)))

(event EventTick
  (params (DeltaSeconds :type Float%20%28single-precision%29)))

(fn ConstructionScript)

(fn GenerarUnidades
  (bind _returnvalue (Transformation|GetActorLocation))
  (bind _bp_civ (Variables|Default|GetBP_Civ))
  (bind _haycapacidad (Default|HayCapacidadDePoblacion (Variables|Default|GetBP_Civ)))
  (if _haycapacidad
    (bind _returnvalue_2 (Game|SpawnActorfromClass "/Game/Blueprints/Mundo/NPC/BP_NPCBase.BP_NPCBase_C" (Math|Transform|MakeTransform (Math|Vector|MakeVector (- (.x _returnvalue) 5e+02) (.y _returnvalue) (.z _returnvalue)) "0,180.000000, 0" "1,1,1") "AdjustIfPossibleButDontSpawnIfColliding" 0 "NewEnumerator1" false 0))
    (Utilities|IsValid _returnvalue_2
      (:Is%20Valid
        (bind _output_get (Variables|Default|SetNPC_BaseAux _returnvalue_2))
        (Default|IngresarCivilizacion _output_get (Variables|Default|Getcivilizacion))
        (Default|ModificarEstadisticas _bp_civ 1 0 0 0.0)
        (Default|AnadirNPCALista _bp_civ (Variables|Default|GetNPC_BaseAux))))))

(fn InicializarCiv
  (bind _asgame_instance_cr (|SeObtieneGameInstanceCR))
  (bind _bp_civilizacion (Default|BuscarCivilizacion _asgame_instance_cr (Variables|Default|Getcivilizacion)))
  (bind _output_get (Variables|Default|SetBP_Civ _bp_civilizacion))
  (Default|ModificarEstadisticas _output_get 0 (Variables|Default|GetaumentoPoblacion) 0 0.0)
  (Utilities|Time|SetTimerbyFunctionName 0 "GenerarUnidades" (Variables|Default|GettiempoEsperaUnidad) true))