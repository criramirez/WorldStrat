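; BP_Casa is a house building that raises the population capacity of the civilization it belongs to.
; On BeginPlay, after the parent logic, it searches the civilization list on GameInstanceCR for entries matching its own Civilizacion.
; For a match it stores the reference, adds AumentoPoblacion to population capacity through ModificarEstadisticas, and registers itself as a building with AnadirEdificio.
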(event EventBeginPlay
  (|CallParentFunction)
  (bind _asgame_instance_cr (Utilities|Casting|CastToGameInstanceCR (Game|GetGameInstance)))
  (for _array_element (Variables|/Game/Blueprints/BpGeneral/GameInstanceCR.GameInstanceCR_C|GetBP_Civilizacion _asgame_instance_cr)
    (if (Utilities|Enum|Equal(Enum) (.civilizacion (Variables|/Game/Blueprints/Mundo/BP_Civilizacion.BP_Civilizacion_C|GetEST_Civi _array_element)) (Variables|Default|Getcivilizacion))
      (bind _output_get (Variables|Default|SetBP_Civ _array_element))
      (Default|ModificarEstadisticas _output_get 0 (Variables|Default|GetaumentoPoblacion) 0 0.0)
      (Default|AnadirEdificio _output_get self))))

(event Collision|EventActorBeginOverlap
  (params (OtherActor :type Actor%20Object%20Reference))
  (|CallParentFunction OtherActor) ; This node is disabled and will not be called.\nDrag off pins to build functionality.
)

(event EventTick
  (params (DeltaSeconds :type Float%20%28single-precision%29))
  (|CallParentFunction DeltaSeconds) ; This node is disabled and will not be called.\nDrag off pins to build functionality.
)

(fn ConstructionScript
  (|CallParentFunction))