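; Resource spawner that scatters a set number of RecursoSpawn actors inside a box volume (Generador, sized in the construction script) at BeginPlay.
; Each spawn starts at a random point in the box and traces straight down for an actor or component tagged "terreno".
; On a hit it snaps to the ground, stores that location in its ESTObjeto struct, gets the spawner's name as a tag and is counted; otherwise it is destroyed without retry.
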(event Custom|verificarRecurso
  (for _index (range 0 (- (Variables|Spawner|GetcantidadRecursos) 1))
    (CallFunction|SpawnRecurso)))

(event EventBeginPlay
  (CallFunction|VerificarRecurso)
  (Actor|GetAllActorswithTag (Utilities|String|StringToName (Utilities|GetDisplayName self))))

(fn ConstructionScript
  (Components|Box|SetBoxExtent (Variables|Default|Getgenerador) (Variables|Spawner|GettamanioSpawner) true))

(fn SpawnRecurso
  (bind _generador (Variables|Default|GetGenerador))
  (bind _returnvalue (Game|SpawnActorfromClass (Variables|Spawner|GetrecursoSpawn) (Math|Transform|MakeTransform (Math|Random|RandomPointinBoundingBox (Transformation|GetWorldLocation _generador) (Variables|/Script/Engine.BoxComponent|GetBoxExtent _generador)) "0, 0, 0" "1,1,1") "AdjustIfPossibleButAlwaysSpawn" 0 true 0))
  (bind _output_get (Variables|Spawner|SetrecursoAux _returnvalue))
  (Utilities|IsValid _output_get
    (:Is%20Valid
      (bind (_outhit _returnvalue_2) (Collision|LineTraceByChannel (Transformation|GetWorldLocation (Variables|/Game/Blueprints/Mundo/Objetos/BP_ObjetoRecurso.BP_ObjetoRecurso_C|GetMallaRecurso _output_get)) (Math|Vector|MakeVector (.X (Math|Vector|BreakVector (Transformation|GetWorldLocation (Variables|/Game/Blueprints/Mundo/Objetos/BP_ObjetoRecurso.BP_ObjetoRecurso_C|GetMallaRecurso _output_get)))) (.Y (Math|Vector|BreakVector (Transformation|GetWorldLocation (Variables|/Game/Blueprints/Mundo/Objetos/BP_ObjetoRecurso.BP_ObjetoRecurso_C|GetMallaRecurso _output_get)))) -1.5e+09) "TraceTypeQuery1" false (Utilities|Array|MakeArray _output_get) "None"))
      (if _returnvalue_2
        (if (Utilities|IsValid (.hitactor _outhit))
          (if (!= (Utilities|Array|FindItem (Variables|/Script/Engine.Actor|GetTags (.hitactor _outhit)) "terreno") -1)
            (Variables|/Game/Blueprints/Mundo/Objetos/BP_Objeto.BP_Objeto_C|SetEST_Objeto (Variables|Spawner|GetrecursoAux) (Utilities|Struct|MakeEST_Objeto (.nombre (Variables|/Game/Blueprints/Mundo/Objetos/BP_Objeto.BP_Objeto_C|GetEST_Objeto (Variables|Spawner|GetrecursoAux))) (.imagen (Variables|/Game/Blueprints/Mundo/Objetos/BP_Objeto.BP_Objeto_C|GetEST_Objeto (Variables|Spawner|GetrecursoAux))) (.apilable (Variables|/Game/Blueprints/Mundo/Objetos/BP_Objeto.BP_Objeto_C|GetEST_Objeto (Variables|Spawner|GetrecursoAux))) (.maxapilable (Variables|/Game/Blueprints/Mundo/Objetos/BP_Objeto.BP_Objeto_C|GetEST_Objeto (Variables|Spawner|GetrecursoAux))) (.peso (Variables|/Game/Blueprints/Mundo/Objetos/BP_Objeto.BP_Objeto_C|GetEST_Objeto (Variables|Spawner|GetrecursoAux))) (.cantidad (Variables|/Game/Blueprints/Mundo/Objetos/BP_Objeto.BP_Objeto_C|GetEST_Objeto (Variables|Spawner|GetrecursoAux))) (Math|Transform|MakeTransform (.impactpoint _outhit) (.rotation (.transformobjeto (Variables|/Game/Blueprints/Mundo/Objetos/BP_Objeto.BP_Objeto_C|GetEST_Objeto (Variables|Spawner|GetrecursoAux)))) (.scale (.transformobjeto (Variables|/Game/Blueprints/Mundo/Objetos/BP_Objeto.BP_Objeto_C|GetEST_Objeto (Variables|Spawner|GetrecursoAux))))) (.clase (Variables|/Game/Blueprints/Mundo/Objetos/BP_Objeto.BP_Objeto_C|GetEST_Objeto (Variables|Spawner|GetrecursoAux))) "(id_2_37FEAA9247A6DE3246C072B4BAF9C72C=0,vida_5_36995D00462D2A93086B4597A89CAA14=0.000000)") :!label _label)
            (Transformation|SetActorLocation (Variables|Spawner|GetrecursoAux) (.impactpoint _outhit) false false)
            (Utilities|Array|Add (Variables|/Script/Engine.Actor|GetTags (Variables|Spawner|GetrecursoAux)) (Utilities|String|StringToName (Utilities|GetDisplayName self)))
            (bind _result (Math|Integer|IncrementInt (Variables|Spawner|GetrecursosCreados))
              (:%20%20
                (Variables|Spawner|SetrecursosCreados _result)))
            (else
              (if (!= (Utilities|Array|FindItem (Variables|/Script/Engine.ActorComponent|GetComponentTags (.hitcomponent _outhit)) "terreno") -1) :!label _label_2
                (goto _label)
                (else
                  (Actor|DestroyActor (Variables|Spawner|GetrecursoAux) :!label _label_3)))))
          (else
            (goto _label_2)))
        (else
          (goto _label_3))))))