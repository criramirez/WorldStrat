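; Clickable resource object in the world that hands itself to the player's ship, BP_NaveCR, when clicked or touched.
; On click or touch, it disables mesh physics and collision, then calls RecursoClic on the ship.
; When Aleatorio is set, construction randomizes scale and yaw, resizes the box to mesh bounds and scales ESTObjeto weight and quantity by size.
; ModificarPeso adjusts weight only while the result stays positive.
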(event OnClicked(MallaRecurso)
  (params (TouchedComponent :type Primitive%20Component%20Object%20Reference) (ButtonPressed :type Key%20Structure))
  (bind _mallarecurso (Variables|Default|GetMallaRecurso))
  (Physics|SetSimulatePhysics _mallarecurso false)
  (Collision|SetCollisionEnabled _mallarecurso "NoCollision")
  (bind _asbp_nave_cr (Utilities|Casting|CastToBP_NaveCR (Game|Player|GetPlayerPawn 0)))
  (Default|RecursoClic _asbp_nave_cr self))

(event OnInputTouchBegin(MallaRecurso)
  (params (FingerIndex :type ETouchIndex%20Enum :default "Touch1") (TouchedComponent :type Primitive%20Component%20Object%20Reference))
  (bind _mallarecurso (Variables|Default|GetMallaRecurso))
  (Physics|SetSimulatePhysics _mallarecurso false)
  (Collision|SetCollisionEnabled _mallarecurso "NoCollision")
  (bind _asbp_nave_cr (Utilities|Casting|CastToBP_NaveCR (Game|Player|GetPlayerPawn 0)))
  (Default|RecursoClic _asbp_nave_cr self))

(event EventBeginPlay
  (|CallParentFunction))

(event Collision|EventActorBeginOverlap
  (params (OtherActor :type Actor%20Object%20Reference))
  (|CallParentFunction OtherActor) ; This node is disabled and will not be called.\nDrag off pins to build functionality.
)

(event EventTick
  (params (DeltaSeconds :type Float%20%28single-precision%29))
  (|CallParentFunction DeltaSeconds))

(fn ConstructionScript
  (|CallParentFunction)
  (CallFunction|EscalaRotacionAlea))

(fn EscalaRotacionAlea
  (bind _returnvalue (Transformation|GetActorScale3D))
  (if (Variables|Default|GetAleatorio)
    (Transformation|SetActorScale3D (Math|Conversions|ToVector(Float) (/ (Math|Conversions|ToFloat(Integer) (Math|Random|RandomIntegerinRange 2 10)) 1e+01)))
    (Components|Box|SetBoxExtent (Variables|Default|GetBox) (.Max (Components|StaticMesh|GetLocalBounds (Variables|Default|GetMallaRecurso))) true)
    (Variables|Default|SetEST_Objeto (Utilities|Struct|MakeEST_Objeto (.nombre (Variables|Default|GetEST_Objeto)) (.imagen (Variables|Default|GetEST_Objeto)) (.apilable (Variables|Default|GetEST_Objeto)) (.maxapilable (Variables|Default|GetEST_Objeto)) (* (.peso (Variables|Default|GetEST_Objeto)) (Math|Float|Truncate (* (.X (Math|Vector|BreakVector _returnvalue)) 1e+01))) (* (.cantidad (Variables|Default|GetEST_Objeto)) (* (.peso (Variables|Default|GetEST_Objeto)) (Math|Float|Truncate (* (.X (Math|Vector|BreakVector _returnvalue)) 1e+01)))) (Math|Transform|MakeTransform (.location (.transformobjeto (Variables|Default|GetEST_Objeto))) (.rotation (.transformobjeto (Variables|Default|GetEST_Objeto))) _returnvalue) (.clase (Variables|Default|GetEST_Objeto)) "(id_2_37FEAA9247A6DE3246C072B4BAF9C72C=0,vida_5_36995D00462D2A93086B4597A89CAA14=0.000000)"))
    (Transformation|SetActorRotation (Math|Rotator|MakeRotator 0.0 0.0 (.yaw (Math|Random|RandomRotator true))))))

(fn ModificarPeso
  (params (Valor :type Integer))
  (bind _self self)
  (if (not (<= (+ (.peso (Variables|Default|GetEST_Objeto _self)) Valor) 0))
    (Variables|Default|SetEST_Objeto _self (Utilities|Struct|MakeEST_Objeto (.nombre (Variables|Default|GetEST_Objeto _self)) (.imagen (Variables|Default|GetEST_Objeto _self)) (.apilable (Variables|Default|GetEST_Objeto _self)) (.maxapilable (Variables|Default|GetEST_Objeto _self)) (+ (.peso (Variables|Default|GetEST_Objeto _self)) Valor) (.cantidad (Variables|Default|GetEST_Objeto _self)) (.transformobjeto (Variables|Default|GetEST_Objeto _self)) (.clase (Variables|Default|GetEST_Objeto _self)) (.est_npc (Variables|Default|GetEST_Objeto _self))))))