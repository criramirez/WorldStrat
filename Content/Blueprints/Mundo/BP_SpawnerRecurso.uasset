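; Resource spawner that scatters RecursoSpawn actors over terrain inside a box volume when play begins.
; The construction script sizes the Generador box from TamanioSpawner, and BeginPlay makes CantidadRecursos spawn attempts at random points within it.
; Each actor line-traces downward, snapping its mesh onto components tagged "terreno" and incrementing RecursosCreados.
; Failed placements are destroyed without retry, so fewer resources may remain than requested.
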(event Custom|verificarRecurso
  (for _index (range 0 (- (Variables|Default|GetcantidadRecursos) 1))
    (CallFunction|SpawnRecurso)))

(event EventBeginPlay
  (CallFunction|VerificarRecurso))

(fn ConstructionScript
  (Components|Box|SetBoxExtent (Variables|Default|Getgenerador) (Variables|Default|GettamanioSpawner) true))

(fn SpawnRecurso
  (bind _generador (Variables|Default|GetGenerador))
  (bind _returnvalue (Game|SpawnActorfromClass :Class (Variables|Default|GetrecursoSpawn) :SpawnTransform (Math|Transform|MakeTransform (Math|Random|RandomPointinBoundingBox (Transformation|GetWorldLocation _generador) (Variables|/Script/Engine.BoxComponent|GetBoxExtent _generador)) "0, 0, 0" "1,1,1") :CollisionHandlingOverride "AdjustIfPossibleButAlwaysSpawn" :Instigator 0))
  (bind _output_get (Variables|Default|SetrecursoAux _returnvalue))
  (Utilities|IsValid _output_get
    (:Is%20Valid
      (bind (_outhit _returnvalue_2) (Collision|LineTraceByChannel (Transformation|GetWorldLocation (Variables|/Game/Blueprints/Mundo/BP_Recurso.BP_Recurso_C|GetMesh _output_get)) (Math|Vector|MakeVector (.X (Math|Vector|BreakVector (Transformation|GetWorldLocation (Variables|/Game/Blueprints/Mundo/BP_Recurso.BP_Recurso_C|GetMesh _output_get)))) (.Y (Math|Vector|BreakVector (Transformation|GetWorldLocation (Variables|/Game/Blueprints/Mundo/BP_Recurso.BP_Recurso_C|GetMesh _output_get)))) -1.5e+04) "TraceTypeQuery1" false (Utilities|Array|MakeArray _output_get) "None"))
      (if _returnvalue_2
        (if (!= (Utilities|Array|FindItem (Variables|/Script/Engine.ActorComponent|GetComponentTags (.hitcomponent _outhit)) "terreno") -1)
          (Transformation|SetWorldLocation (Variables|/Game/Blueprints/Mundo/BP_Recurso.BP_Recurso_C|GetMesh (Variables|Default|GetrecursoAux)) (.impactpoint _outhit) false false)
          (bind _result (Math|Integer|IncrementInt (Variables|Default|GetrecursosCreados))
            (:%20%20
              (Variables|Default|SetrecursosCreados _result)))
          (else
            (Actor|DestroyActor (Variables|Default|GetrecursoAux) :!label _label)))
        (else
          (goto _label))))))