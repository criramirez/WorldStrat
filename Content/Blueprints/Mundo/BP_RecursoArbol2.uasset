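; BP_RecursoArbol2 is a tree resource Blueprint that randomizes its weight and shape, inheriting all other behavior from its parent.
; After the parent construction script, it sets Peso to PesoRecurso times a random factor, truncated to a whole number.
; It then scales the mesh's world size randomly and non-uniformly per axis, with rolls independent of the weight.
; The event graph adds no active logic beyond calling the parent BeginPlay.
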(event EventBeginPlay
  (|CallParentFunction))

(event Collision|EventActorBeginOverlap
  (params (OtherActor :type Actor%20Object%20Reference))
  (|CallParentFunction OtherActor) ; This node is disabled and will not be called.\nDrag off pins to build functionality.
)

(event EventTick
  (params (DeltaSeconds :type Float%20%28single-precision%29))
  (|CallParentFunction DeltaSeconds) ; This node is disabled and will not be called.\nDrag off pins to build functionality.
)

(fn ConstructionScript
  (bind _returnvalue (Math|Random|RandomFloatinRange 0.3 1.0))
  (|CallParentFunction)
  (Variables|Default|Setpeso (Math|Conversions|ToFloat(Integer) (Math|Float|Truncate (* _returnvalue (Variables|Default|GetpesoRecurso)))))
  (Transformation|SetWorldScale3D (Variables|Character|GetMesh) (Math|Vector|MakeVector _returnvalue _returnvalue _returnvalue)))