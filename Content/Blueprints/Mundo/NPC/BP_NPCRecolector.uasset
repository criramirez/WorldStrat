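; Gatherer NPC that harvests wood or food from a selected object into a capacity-limited inventory.
; Recolectar starts a looping timer if none is running and the inventory is not full.
; Recoleccion reduces the object's weight and adds to the matching resource, stopping the timer and flagging the inventory full at the limit; both resources are checked against wood capacity.
; VaciarInventario zeroes both amounts and clears the full flag.
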(event EventBeginPlay
  (|CallParentFunction) ; This node is disabled and will not be called.\nDrag off pins to build functionality.
)

(event Collision|EventActorBeginOverlap
  (params (OtherActor :type Actor%20Object%20Reference)))

(event EventTick
  (params (DeltaSeconds :type Float%20%28single-precision%29))
  (|CallParentFunction DeltaSeconds) ; This node is disabled and will not be called.\nDrag off pins to build functionality.
)

(fn ConstructionScript
  (|CallParentFunction))

(fn Recolectar
  (if (Utilities|Time|IsValidTimerHandle (Variables|Default|GetTimer%20de%20recoleccion))
    _
    (elif (Variables|Default|GetInventarioLleno)
      _
      (else
        (bind _returnvalue (Utilities|Time|SetTimerbyEvent (EventDispatchers|CreateEvent :!event Recoleccion) 2.0 true))
        (Variables|Default|SetTimer%20de%20recoleccion _returnvalue)
        (Variables|Default|Setrecolectando true)
        (return false))))
  (return (Variables|Default|GetInventarioLleno)))

(fn Recoleccion
  (bind _objetoseleccionado (Variables|Default|GetObjetoSeleccionado))
  (bind _catidadrecoleccion (Variables|Default|GetCatidadRecoleccion))
  (Default|ModificarPeso _objetoseleccionado (* (Variables|Default|GetCatidadRecoleccion) -1))
  (switch Utilities|FlowControl|Switch|SwitchonENUM_TipoDeRecurso (Variables|/Game/Blueprints/Mundo/Objetos/BP_ObjetoRecurso.BP_ObjetoRecurso_C|GetTipo _objetoseleccionado)
    (:NewEnumerator0
      (if (>= (+ (.madera (Variables|Default|GetInventario)) _catidadrecoleccion) (.capacidadmadera (Variables|Default|GetInventario)))
        (Variables|Default|SetInventario (Utilities|Struct|MakeEST_InventarioNPCRecolector (.capacidadmadera (Variables|Default|GetInventario)) (.comida (Variables|Default|GetInventario)) (.capacidadcomida (Variables|Default|GetInventario)) (.capacidadmadera (Variables|Default|GetInventario))))
        (Variables|Default|SetInventarioLleno true :!label _label)
        (Variables|Default|Setrecolectando false)
        (Utilities|Time|ClearandInvalidateTimerbyHandle (Variables|Default|GetTimer%20de%20recoleccion))
        (else
          (Variables|Default|SetInventario (Utilities|Struct|MakeEST_InventarioNPCRecolector (+ (.madera (Variables|Default|GetInventario)) _catidadrecoleccion) (.comida (Variables|Default|GetInventario)) (.capacidadmadera (Variables|Default|GetInventario)) (.capacidadcomida (Variables|Default|GetInventario)))))))
    (:NewEnumerator1
      (if (>= (+ (.comida (Variables|Default|GetInventario)) _catidadrecoleccion) (.capacidadmadera (Variables|Default|GetInventario)))
        (Variables|Default|SetInventario (Utilities|Struct|MakeEST_InventarioNPCRecolector (.madera (Variables|Default|GetInventario)) (.capacidadcomida (Variables|Default|GetInventario)) (.capacidadmadera (Variables|Default|GetInventario)) (.capacidadcomida (Variables|Default|GetInventario))))
        (goto _label)
        (else
          (Variables|Default|SetInventario (Utilities|Struct|MakeEST_InventarioNPCRecolector (.madera (Variables|Default|GetInventario)) (+ (.comida (Variables|Default|GetInventario)) _catidadrecoleccion) (.capacidadmadera (Variables|Default|GetInventario)) (.capacidadcomida (Variables|Default|GetInventario)))))))))

(fn VaciarInventario
  (Variables|Default|SetInventario (Utilities|Struct|MakeEST_InventarioNPCRecolector 0 0 (.capacidadmadera (Variables|Default|GetInventario)) (.capacidadcomida (Variables|Default|GetInventario))))
  (Variables|Default|SetInventarioLleno false))