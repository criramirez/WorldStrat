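; BP_Civilizacion holds the state of one civilization in an ESTCivi struct: population, population limit, food, NPCs and buildings.
; ModificarEstadisticas adds deltas to population, limit and food, though its Madera (wood) input is unused.
; AnadirNPCALista and AnadirEdificio register NPCs and buildings in the struct's lists.
; HayCapacidadDePoblacion and CuentaConLosRecusos check for free population capacity and enough food; the event graph is empty.
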(event EventBeginPlay)

(event Collision|EventActorBeginOverlap
  (params (OtherActor :type Actor%20Object%20Reference)))

(event EventTick
  (params (DeltaSeconds :type Float%20%28single-precision%29)))

(fn ConstructionScript)

(fn ModificarEstadisticas
  (params (Poblacion :type Integer) (CapacidadPoblacion :type Integer) (Alimento :type Integer) (Madera :type Float%20%28single-precision%29))
  (Variables|Default|SetEST_Civi (Utilities|Struct|MakeEST_Civilizacion (.civilizacion (Variables|Default|GetEST_Civi)) (+ (.poblacion (Variables|Default|GetEST_Civi)) Poblacion) (+ CapacidadPoblacion (.limitepoblacion (Variables|Default|GetEST_Civi))) (+ Alimento (.comida (Variables|Default|GetEST_Civi))) (.npcs (Variables|Default|GetEST_Civi)) (.edificios (Variables|Default|GetEST_Civi)))))

(fn AnadirNPCALista
  (params (NPC :type BP%20NPC%20Base%20Object%20Reference))
  (Utilities|Array|Add (.npcs (Variables|Default|GetEST_Civi)) NPC)
  (Variables|Default|SetEST_Civi (Utilities|Struct|MakeEST_Civilizacion (.civilizacion (Variables|Default|GetEST_Civi)) (.poblacion (Variables|Default|GetEST_Civi)) (.limitepoblacion (Variables|Default|GetEST_Civi)) (.comida (Variables|Default|GetEST_Civi)) (.npcs (Variables|Default|GetEST_Civi)) (.edificios (Variables|Default|GetEST_Civi)))))

(fn HayCapacidadDePoblacion
  (bind _est_civi (Variables|Default|GetEST_Civi))
  (return (< (.poblacion _est_civi) (.limitepoblacion _est_civi))))

(fn AnadirEdificio
  (params (Edificio :type Actor%20Object%20Reference))
  (Utilities|Array|Add (.edificios (Variables|Default|GetEST_Civi)) Edificio)
  (Variables|Default|SetEST_Civi (Utilities|Struct|MakeEST_Civilizacion (.civilizacion (Variables|Default|GetEST_Civi)) (.poblacion (Variables|Default|GetEST_Civi)) (.limitepoblacion (Variables|Default|GetEST_Civi)) (.comida (Variables|Default|GetEST_Civi)) (.npcs (Variables|Default|GetEST_Civi)) (.edificios (Variables|Default|GetEST_Civi)))))

(fn CuentaConLosRecusos
  (params (Comida :type Integer))
  (return (<= Comida (.comida (Variables|Default|GetEST_Civi)))))