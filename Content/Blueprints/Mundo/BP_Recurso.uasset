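; BP_Recurso is a resource actor with a weight (Peso) that can be removed from the world and later respawned.
; Destruir saves the mesh reference, destroys the component and teleports the actor out of the way, keeping it alive.
; Reconstruir spawns a fresh actor of the same class at a given transform, passes on Peso, enables mesh physics and destroys the old actor.
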(event Custom|Destruir
  (bind _mesh (Variables|Default|GetMesh))
  (Variables|Default|SetmeshAnterior _mesh)
  (Components|DestroyComponent _mesh)
  (Transformation|SetActorLocation "-1000.000000,-1000.000000,-1000.000000" false false))

(event Custom|Reconstruir
  (params (transformNueva :type Transform))
  (bind _returnvalue (Game|SpawnActorfromClass (Utilities|GetClass self) transformNueva "Undefined" 0 0))
  (CallFunction|SetVariablesRecurso _returnvalue (Variables|Default|Getpeso))
  (Physics|SetSimulatePhysics (Variables|BP_Recurso_C|GetMesh _returnvalue) true)
  (Actor|DestroyActor))

(event EventBeginPlay)

(event Collision|EventActorBeginOverlap
  (params (OtherActor :type Actor%20Object%20Reference)))

(event EventTick
  (params (DeltaSeconds :type Float%20%28single-precision%29)))

(fn ConstructionScript)