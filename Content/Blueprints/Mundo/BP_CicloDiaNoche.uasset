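; BP_CicloDiaNoche is an actor that drives a looping day-night cycle by rotating the Sol light.
; Each tick it accumulates Tiempo, resets it on reaching DuracionCiclo, and maps it to a negative pitch covering one full turn per cycle.
; After each rotation it calls UpdateSunDirection on DireccionSol to sync the sun direction; the node zeroing the light's intensity never runs.
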(event EventBeginPlay)

(event Collision|EventActorBeginOverlap
  (params (OtherActor :type Actor%20Object%20Reference)))

(event EventTick
  (params (DeltaSeconds :type Float%20%28single-precision%29))
  (if (>= (+ DeltaSeconds (Variables|Default|GetTiempo)) (Variables|Default|GetDuracion%20Ciclo))
    (Variables|Default|SetTiempo 0.0)
    (else
      (Variables|Default|SetTiempo (+ DeltaSeconds (Variables|Default|GetTiempo)))
      (Transformation|SetActorRotation (Variables|Default|GetSol) (Math|Rotator|MakeRotator 0.0 (- 0.0 (/ (* (Variables|Default|GetTiempo) 9e+01) (/ (Variables|Default|GetDuracion%20Ciclo) 4.0))) 0.0))
      (Default|UpdateSunDirection (Variables|Default|GetDireccion%20Sol)))))

(fn ConstructionScript)