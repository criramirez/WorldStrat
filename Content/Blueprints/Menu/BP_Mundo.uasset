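; BP_Mundo is a menu globe actor that spins and lets the player pick South America or Africa to load that region's level.
; A timeline started on BeginPlay feeds its rotation value into Rotar, which adds local yaw while EstaRotando is set.
; Clicking or touching a continent sets the map name and, if Activo, shows the HUD_Carga loading widget, then opens the level after a short delay.
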(event OnClicked(americaSur)
  (params (TouchedComponent :type Primitive%20Component%20Object%20Reference) (ButtonPressed :type Key%20Structure))
  (Variables|Default|Setmapa "MapaRamirez")
  (if (Variables|Default|Getactivo)
    (bind _returnvalue (UserInterface|CreateWidget "/Game/Blueprints/UI/HUD_Carga.HUD_Carga_C" (Game|GetPlayerController 0)))
    (UserInterface|Viewport|AddtoViewport _returnvalue 0)
    (Utilities|FlowControl|Delay 1.0)
    (Game|OpenLevel(byName) (Utilities|String|StringToName (Variables|Default|Getmapa)))))

(event OnInputTouchBegin(americaSur)
  (params (FingerIndex :type ETouchIndex%20Enum :default "Touch1") (TouchedComponent :type Primitive%20Component%20Object%20Reference))
  (Variables|Default|Setmapa "MapaRamirez")
  (if (Variables|Default|Getactivo)
    (bind _returnvalue (UserInterface|CreateWidget "/Game/Blueprints/UI/HUD_Carga.HUD_Carga_C" (Game|GetPlayerController 0)))
    (UserInterface|Viewport|AddtoViewport _returnvalue 0)
    (Utilities|FlowControl|Delay 1.0)
    (Game|OpenLevel(byName) (Utilities|String|StringToName (Variables|Default|Getmapa)))))

(event OnClicked(africa)
  (params (TouchedComponent :type Primitive%20Component%20Object%20Reference) (ButtonPressed :type Key%20Structure))
  (Variables|Default|Setmapa "Mapa1Africa")
  (if (Variables|Default|Getactivo)
    (bind _returnvalue (UserInterface|CreateWidget "/Game/Blueprints/UI/HUD_Carga.HUD_Carga_C" (Game|GetPlayerController 0)))
    (UserInterface|Viewport|AddtoViewport _returnvalue 0)
    (Utilities|FlowControl|Delay 1.0)
    (Game|OpenLevel(byName) (Utilities|String|StringToName (Variables|Default|Getmapa)))))

(event OnInputTouchBegin(africa)
  (params (FingerIndex :type ETouchIndex%20Enum :default "Touch1") (TouchedComponent :type Primitive%20Component%20Object%20Reference))
  (Variables|Default|Setmapa "Mapa1Africa")
  (if (Variables|Default|Getactivo)
    (bind _returnvalue (UserInterface|CreateWidget "/Game/Blueprints/UI/HUD_Carga.HUD_Carga_C" (Game|GetPlayerController 0)))
    (UserInterface|Viewport|AddtoViewport _returnvalue 0)
    (Utilities|FlowControl|Delay 1.0)
    (Game|OpenLevel(byName) (Utilities|String|StringToName (Variables|Default|Getmapa)))))

(event EventBeginPlay
  (Utilities|FlowControl|Sequence
    (:then_0
      (bind _rotacion (Timeline|TiempoRotarTierra Play)
        (:Update
          (CallFunction|Rotar _rotacion))))))

(fn ConstructionScript)

(fn Rotar
  (params (rotar%20z :type Float%20%28single-precision%29))
  (if (Variables|Default|GetestaRotando)
    (Transformation|AddActorLocalRotation (Math|Rotator|MakeRotator 0.0 0.0 rotar%20z) false false)))