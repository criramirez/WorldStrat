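; Prototype player actor that moves from axis input and abducts ("aducir") objects picked with the mouse.
; Tick applies clamped, speed-scaled input as a swept world offset and turns the Base component to face the movement direction.
; Left click sets the Aduccion flag and stores the object found by BuscarObjetoConMouse.
; While flagged, Tick calls Aduccir, which runs Encojer (shrink) on that object toward the actor's transform until its result clears the flag.
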(event Custom|aduccir
  ;[1 1 1] se aducce, se realiza una animacion.
  (bind _no_ejecutar (CallFunction|Encojer (Transformation|GetActorTransform) (stale Input|MouseEvents|LeftMouseButton _actorselecionado) (* (stale EventTick DeltaSeconds) (Variables|Default|GetvelocidadAduccion))))
  (Variables|Default|SetAduccion _no_ejecutar))

(event EventTick
  (params (DeltaSeconds :type Float%20%28single-precision%29))
  (bind _returnvalue (Input|AxisValues|GetHorizontal))
  (bind _returnvalue_2 (Input|AxisValues|GetVertical))
  (bind _velocidad (Variables|Default|GetVelocidad))
  (bind _returnvalue_3 (Math|Vector|MakeVector _returnvalue_2 _returnvalue 0.0))
  (bind _returnvalue_4 (* DeltaSeconds _velocidad))
  (bind _returnvalue_5 (Math|Vector|ClampVectorSize _returnvalue_3 0.0 1.0))
  (bind _returnvalue_6 (* _returnvalue_5 _returnvalue_4))
  (Utilities|FlowControl|Sequence
    (:then_0
      ;[1 1 1] Movimiento y rotacion
      (if (> (Math|Vector|VectorLength _returnvalue_6) 0.0)
        (Transformation|SetWorldRotation (Variables|Default|Getbase) (Math|Conversions|RotationFromXVector _returnvalue_6) false false)
        (Transformation|AddActorWorldOffset _returnvalue_6 true)))
    (:then_1
      (if (Variables|Default|GetAduccion)
        (CallFunction|Aduccir)))))

(event Input|MouseEvents|LeftMouseButton
  (params (Key :type Key%20Structure))
  ;[1 1 1] dispara el evento aduccir y busca el objevto a aduccir
  (:Pressed
    (Variables|Default|SetAduccion true)
    (bind _actorselecionado (CallFunction|BuscarObjetoConMouse))
    (Variables|Default|SetObjectoAducido _actorselecionado)))

(fn ConstructionScript)