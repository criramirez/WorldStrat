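; Player-controlled ship that moves on the horizontal plane and abducts resources into a weight-limited cargo hold.
; Tick drives swept, input-facing movement and, after a left click picks a target, repeatedly calls Encojer to shrink it toward the ship.
; Resources that fit are stored in Bodega and destroyed, and cargo weight reduces speed.
; Holding X repairs health through a delayed loop; Z, Q and Y are apparent debug keys.
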(event Custom|aduccir
  ;[1 1 1] se aducce, se realiza una animacion.
  (bind _no_ejecutar (CallFunction|Encojer (Transformation|GetActorTransform) (Variables|Default|Getrecurso) (* (stale EventTick DeltaSeconds) (Variables|Default|GetvelocidadAduccion))))
  (bind _output_get (Variables|Default|SetAduccion _no_ejecutar))
  (if (not _output_get)
    (bind (_anadido _pesoactual) (CallFunction|VerificarCapacidadBodega (Variables|Default|Getrecurso)))
    (CallFunction|ReduccionVelocidad _pesoactual)
    (Development|PrintString (Utilities|String|ToString(Float) (Variables|Default|GetVelocidad)))
    (if _anadido
      (Default|Destruir (Variables|Default|Getrecurso)))))

(event EventBeginPlay)

(event Collision|EventActorBeginOverlap
  (params (OtherActor :type Actor%20Object%20Reference)))

(event EventTick
  (params (DeltaSeconds :type Float%20%28single-precision%29))
  (bind _recurso (Variables|Default|Getrecurso))
  (Utilities|FlowControl|Sequence
    (:then_0
      (CallFunction|Movimiento DeltaSeconds))
    (:then_1
      (if (Variables|Default|GetAduccion)
        (if (!= _recurso 0)
          (if (== (Utilities|Array|FindItem (Variables|Default|Getbodega) _recurso) -1)
            (CallFunction|Aduccir)))))))

(event Input|MouseEvents|LeftMouseButton
  (params (Key :type Key%20Structure))
  (:Pressed
    ;[1 1 1] dispara el evento aduccir y busca el objevto a aduccir
    (Variables|Default|SetAduccion true)
    (bind _actorselecionado (CallFunction|BuscarObjetoConMouse))
    (Variables|Default|Setrecurso _actorselecionado)))

(event Input|KeyboardEvents|Q
  (params (Key :type Key%20Structure))
  (:Pressed
    (for _array_element (Variables|Default|Getbodega)
      (Development|PrintString (Utilities|String|ToString(Float) (Variables|/Game/Blueprints/Mundo/BP_Recurso.BP_Recurso_C|Getpeso _array_element))))))

(event Input|KeyboardEvents|Z
  (params (Key :type Key%20Structure))
  (:Pressed
    (Variables|Default|Setvida (- (Variables|Default|Getvida) 1.0))))

(event Input|KeyboardEvents|X
  (params (Key :type Key%20Structure))
  (:Pressed
    (Variables|Default|Setreparar true)
    (Utilities|FlowControl|Delay 0.2 :!label _label)
    (CallFunction|Reparacion :!label _label_2)
    (Utilities|FlowControl|Delay (Variables|Default|GettiempoReparacion))
    (goto _label_2))
  (:Released
    (Variables|Default|Setreparar false)
    (goto _label)))

(event Input|KeyboardEvents|Y
  (params (Key :type Key%20Structure))
  (:Pressed
    (CallFunction|VerificarCapacidadBodega (Variables|Default|Getrecurso))))

(fn ConstructionScript
  (Variables|Default|SetvelociddadIni (Variables|Default|GetVelocidad))
  (Variables|Default|Setvida (Variables|Default|GetvidaMaxima)))

(fn VerificarCapacidadBodega
  (params (recurso :type BP%20Recurso%20Object%20Reference))
  (LocalVariables|SetrecursoVerificar recurso)
  (LocalVariables|Setcapacidad (Variables|Default|Getcapacidad_bodega))
  (for _array_element (Variables|Default|Getbodega)
    (LocalVariables|Setcapacidad (- (LocalVariables|Getcapacidad) (Variables|/Game/Blueprints/Mundo/BP_Recurso.BP_Recurso_C|Getpeso _array_element))))
  (bind _output_get (LocalVariables|Setcapacidad (- (LocalVariables|Getcapacidad) (Variables|/Game/Blueprints/Mundo/BP_Recurso.BP_Recurso_C|Getpeso (LocalVariables|GetrecursoVerificar)))))
  (if (< _output_get 0.0)
    (return false (- (Variables|Default|Getcapacidad_bodega) (LocalVariables|Getcapacidad)))
    (else
      (Utilities|Array|Add (Variables|Default|Getbodega) (LocalVariables|GetrecursoVerificar))
      (return true (- (Variables|Default|Getcapacidad_bodega) (LocalVariables|Getcapacidad))))))

(fn Movimiento
  (params (Tiempo :type Float%20%28single-precision%29))
  (bind _returnvalue (Input|AxisValues|GetHorizontal))
  (bind _returnvalue_2 (Input|AxisValues|GetVertical))
  (bind _velocidad (Variables|Default|GetVelocidad))
  (bind _returnvalue_3 (Math|Vector|MakeVector _returnvalue_2 _returnvalue 0.0))
  (bind _returnvalue_4 (* Tiempo _velocidad))
  (bind _returnvalue_5 (Math|Vector|ClampVectorSize _returnvalue_3 0.0 1.0))
  (bind _returnvalue_6 (* _returnvalue_5 _returnvalue_4))
  ;[1 1 1] Movimiento y rotacion
  (if (> (Math|Vector|VectorLength _returnvalue_6) 0.0)
    (Transformation|SetWorldRotation (Variables|Character|GetMesh) (Math|Conversions|RotationFromXVector _returnvalue_6) false false)
    (Transformation|AddActorWorldOffset _returnvalue_6 true)))

(fn Abducir
  (params (Time :type Float%20%28single-precision%29)))

(fn ReduccionVelocidad
  (params (pesoActual :type Float%20%28single-precision%29))
  (if (not (== pesoActual 0.0))
    (bind _output_get (Variables|Default|SetVelocidad (- (Variables|Default|GetvelociddadIni) (* pesoActual (/ (Variables|Default|GetvelociddadIni) 2e+02)))))
    (Development|PrintString (Utilities|String|ToString(Float) _output_get))
    (return)))

(fn Reparacion
  (if (Variables|Default|Getreparar)
    (if (< (Variables|Default|Getvida) (Variables|Default|GetvidaMaxima))
      (bind _result (Math|Float|IncrementFloat (Variables|Default|Getvida))
        (:%20%20
          (Variables|Default|Setvida _result))))))