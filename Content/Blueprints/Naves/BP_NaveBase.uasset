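; Base ship Blueprint that moves and rotates from axis input, abducts resources into a weight-limited hold, and self-repairs while X is held.
; In-range resources picked via BuscarObjetoConMouse join a capped list that Tick processes through Encojer; finished ones are stored and destroyed if they fit.
; Cargo weight lowers speed relative to its initial value.
; The hold feeds a toggleable HUD_Inventario widget, and debug keys print it or reconstruct its first item.
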(event Custom|aduccir
  ;[1 1 1] se aducce, se realiza una animacion.
  (bind (_recurso _com_objectos) (CallFunction|Abducir (Variables|bodega|Getrecurso) (Variables|estadisticas|GetLimiteAbducion)))
  (Variables|bodega|Setrecurso 0)
  (if (!= _recurso 0)
    (Variables|funciones|SetAduccion _com_objectos)
    (Development|PrintString (Utilities|String|Append "objeto a add  " (Utilities|GetDisplayName _recurso) "  condicion  " (Utilities|String|ToString(Boolean) _com_objectos)) true true "(R=0.037376,G=0.000000,B=1.000000,A=1.000000)" 2e+02)
    ;[1 1 1] se agrega a bodega y reduce velocidad
    (bind (_anadido _pesoactual) (CallFunction|VerificarCapacidadBodega _recurso))
    (CallFunction|ReduccionVelocidad _pesoactual)
    ;[1 1 1] si es añadido se elimina
    (Development|PrintString (Utilities|String|ToString(Float) (Variables|estadisticas|GetVelocidad)))
    (if _anadido
      (Default|Destruir _recurso))))

(event Custom|abrirInventario
  (bind _inventario (Variables|bodega|Getinventario))
  ;[1 1 1] Inventario
  (Utilities|FlowControl|FlipFlop
    (:A
      (Widget|SetVisibility _inventario "Visible")
      (Default|ConfigurarInventario (Variables|bodega|Getinventario) (Variables|bodega|Getbodega)))
    (:B
      (Widget|SetVisibility _inventario "Hidden")
      (Widget|SetVisibility (Variables|/Game/Blueprints/UI/HUD_Inventario.HUD_Inventario_C|Getrecurso_info _inventario) "Hidden")
      (Variables|/Game/Blueprints/UI/HUD_Inventario.HUD_Inventario_C|Setinformacion _inventario ""))))

(event EventTick
  (params (DeltaSeconds :type Float%20%28single-precision%29))
  (Utilities|FlowControl|Sequence
    (:then_0
      (CallFunction|Movimiento))
    (:then_1
      (if (Variables|funciones|GetAduccion)
        (CallFunction|Aduccir)))
    (:then_2
      (Variables|estadisticas|SetTiempo DeltaSeconds))))

(event EventBeginPlay
  (bind _foundwidgets (Widget|GetAllWidgetsOfClass "/Game/Blueprints/UI/HUD_Inventario.HUD_Inventario_C" true))
  (Variables|bodega|Setinventario (Utilities|Array|Get(acopy) _foundwidgets)))

(event Input|ActionEvents|InputActionAccionAbducir
  (params (Key :type Key%20Structure))
  ;[1 1 1] dispara el evento aduccir y busca el objevto a aduccir, si se encuentra en el rango lo pasa a la variable
  (:Pressed
    (Variables|funciones|SetAduccion true)
    (bind _actorselecionado (CallFunction|BuscarObjetoConMouse self (Class|KismetInputLibrary|KeyGetDisplayName Key)))
    (if (<= (Transformation|GetDistanceTo _actorselecionado) (Variables|estadisticas|GetRangoAbducion))
      (Development|PrintString "esta en el rango permitido")
      (Variables|bodega|Setrecurso _actorselecionado)
      (else
        (Development|PrintString "fuera del rango")))))

(event Input|ActionEvents|InputActionInventario
  (params (Key :type Key%20Structure))
  ;[1 1 1] Inventario
  (:Pressed
    (CallFunction|AbrirInventario)))

(event Input|KeyboardEvents|K
  (params (Key :type Key%20Structure))
  (bind _returnvalue (Transformation|GetActorTransform))
  (bind _bodega (Variables|bodega|Getbodega))
  (bind _output (Utilities|Array|Get(acopy) _bodega))
  (:Pressed
    (Default|Reconstruir _output (Math|Transform|MakeTransform (+ (.location _returnvalue) "100.000000, 0, 0") (.rotation _returnvalue) (.scale _returnvalue)))
    (Utilities|Array|RemoveItem (Variables|bodega|Getbodega) _output)))

(event Input|KeyboardEvents|Q
  (params (Key :type Key%20Structure))
  ;[1 1 1] muestra loq esta actualmente en bodega
  (:Pressed
    (for _array_element (Variables|bodega|Getbodega)
      (Development|PrintString (Utilities|String|Append (Utilities|GetDisplayName _array_element) (Utilities|String|ToString(Float) (Variables|/Game/Blueprints/Mundo/BP_Recurso.BP_Recurso_C|Getpeso _array_element)))))))

(event Input|KeyboardEvents|X
  (params (Key :type Key%20Structure))
  ;[1 1 1] AutoReparar
  (:Pressed
    (Variables|funciones|Setreparar true)
    (Utilities|FlowControl|Delay 0.2 :!label _label)
    (CallFunction|Reparacion :!label _label_2)
    (Utilities|FlowControl|Delay (Variables|estadisticas|GettiempoReparacion))
    (goto _label_2))
  (:Released
    (Variables|funciones|Setreparar false)
    (goto _label)))

(fn ConstructionScript
  (Variables|estadisticas|SetvelociddadIni (Variables|estadisticas|GetVelocidad))
  (Variables|estadisticas|Setvida (Variables|estadisticas|GetvidaMaxima)))

(fn VerificarCapacidadBodega
  (params (recurso :type BP%20Recurso%20Object%20Reference))
  (LocalVariables|SetrecursoVerificar recurso)
  (LocalVariables|Setcapacidad (Variables|estadisticas|Getcapacidad_bodega))
  (for _array_element (Variables|bodega|Getbodega)
    (LocalVariables|Setcapacidad (- (LocalVariables|Getcapacidad) (Variables|/Game/Blueprints/Mundo/BP_Recurso.BP_Recurso_C|Getpeso _array_element))))
  (bind _output_get (LocalVariables|Setcapacidad (- (LocalVariables|Getcapacidad) (Variables|/Game/Blueprints/Mundo/BP_Recurso.BP_Recurso_C|Getpeso (LocalVariables|GetrecursoVerificar)))))
  (if (< _output_get 0.0)
    (Variables|bodega|SetPesoActual (- (Variables|estadisticas|Getcapacidad_bodega) (LocalVariables|Getcapacidad)))
    (return false (- (Variables|estadisticas|Getcapacidad_bodega) (LocalVariables|Getcapacidad)))
    (else
      (Utilities|Array|Add (Variables|bodega|Getbodega) (LocalVariables|GetrecursoVerificar))
      (Variables|bodega|SetPesoActual (- (Variables|estadisticas|Getcapacidad_bodega) (LocalVariables|Getcapacidad)))
      (return true (- (Variables|estadisticas|Getcapacidad_bodega) (LocalVariables|Getcapacidad))))))

(fn Movimiento
  (bind _returnvalue (Input|AxisValues|GetHorizontal))
  (bind _returnvalue_2 (Input|AxisValues|GetVertical))
  (bind _tiempo (Variables|estadisticas|GetTiempo))
  (bind _velocidad (Variables|estadisticas|GetVelocidad))
  (bind _returnvalue_3 (Math|Vector|MakeVector _returnvalue_2 _returnvalue 0.0))
  (bind _returnvalue_4 (* _tiempo _velocidad))
  (bind _returnvalue_5 (Math|Vector|ClampVectorSize _returnvalue_3 0.0 1.0))
  (bind _returnvalue_6 (* _returnvalue_5 _returnvalue_4))
  ;[1 1 1] Movimiento y rotacion
  (if (> (Math|Vector|VectorLength _returnvalue_6) 0.0)
    (Transformation|SetWorldRotation (Variables|Character|GetMesh) (Math|Conversions|RotationFromXVector _returnvalue_6) false false)
    (Transformation|AddActorWorldOffset _returnvalue_6 true)))

(fn Abducir
  (params (Entrada :type BP%20Recurso%20Object%20Reference) (LimiteObjetos :type Integer))
  (bind _actualabducion (Variables|funciones|GetActualAbducion))
  (bind _actualabducion_2 (Variables|funciones|GetActualAbducion))
  (bind _returnvalue (Utilities|Array|Length _actualabducion_2))
  (bind _returnvalue_2 (== _returnvalue 0))
  (bind _returnvalue_3 (not _returnvalue_2))
  (if (!= Entrada 0)
    (if (and (== (Utilities|Array|FindItem (Variables|funciones|GetActualAbducion) Entrada) -1) (< (Utilities|Array|Length (Variables|funciones|GetActualAbducion)) LimiteObjetos))
      ;[1 1 1] se añade objecto
      (Utilities|Array|Add _actualabducion Entrada)))
  (bind _array_element (Utilities|Array|ForEachLoopwithBreak _actualabducion :!label _label)
    (:LoopBody
      (bind _no_ejecutar (CallFunction|Encojer (Transformation|GetActorTransform) _array_element (* (Variables|estadisticas|GetTiempo) (Variables|estadisticas|GetvelocidadAduccion))))
      (if (not _no_ejecutar)
        (LocalVariables|SetbpRe _array_element)
        (Utilities|Array|RemoveItem (Variables|funciones|GetActualAbducion) _array_element)
        (goto _label Break)))
    (:Completed
      (Utilities|IsValid (LocalVariables|GetbpRe)
        (:Is%20Valid
          (return (LocalVariables|GetbpRe) _returnvalue_3))
        (:Is%20Not%20Valid
          (return 0 _returnvalue_3))))))

(fn ReduccionVelocidad
  (params (pesoActual :type Float%20%28single-precision%29))
  (if (not (== pesoActual 0.0))
    (bind _output_get (Variables|estadisticas|SetVelocidad (- (Variables|estadisticas|GetvelociddadIni) (* pesoActual (/ (Variables|estadisticas|GetvelociddadIni) 2e+02)))))
    (Development|PrintString (Utilities|String|ToString(Float) _output_get))
    (return)))

(fn Reparacion
  (if (Variables|funciones|Getreparar)
    (if (< (Variables|estadisticas|Getvida) (Variables|estadisticas|GetvidaMaxima))
      (bind _result (Math|Float|IncrementFloat (Variables|estadisticas|Getvida))
        (:%20%20
          (Variables|estadisticas|Setvida _result))))))