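; Blueprint function library of getters and setters for a civilization's ESTCivi struct: civilization type, population, population limit, food, NPCs and buildings.
; Getters read one field from the passed civilization Blueprint.
; Each setter rebuilds the whole struct with one field replaced, setting the last two members to zero.
; Only the civilization enum setter writes the struct back; the others return the modified copy.
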(fn SetESTEnumCivilizacion
  (params (enum_civ :type ENUM_Civilizaviones%20Enum :default "NewEnumerator2") (ets_civ :type BP%20Civilizacion%20Object%20Reference))
  (bind _output_get (LocalVariables|Setest_civilizacionModificada (Utilities|Struct|MakeEST_Civilizacion enum_civ (.Poblacion (Utilities|Struct|BreakEST_Civilizacion (Variables|/Game/Blueprints/Mundo/BP_Civilizacion.BP_Civilizacion_C|GetEST_Civi ets_civ))) (.LimitePoblacion (Utilities|Struct|BreakEST_Civilizacion (Variables|/Game/Blueprints/Mundo/BP_Civilizacion.BP_Civilizacion_C|GetEST_Civi ets_civ))) (.Comida (Utilities|Struct|BreakEST_Civilizacion (Variables|/Game/Blueprints/Mundo/BP_Civilizacion.BP_Civilizacion_C|GetEST_Civi ets_civ))) (.npcs (Utilities|Struct|BreakEST_Civilizacion (Variables|/Game/Blueprints/Mundo/BP_Civilizacion.BP_Civilizacion_C|GetEST_Civi ets_civ))) (.Edificios (Utilities|Struct|BreakEST_Civilizacion (Variables|/Game/Blueprints/Mundo/BP_Civilizacion.BP_Civilizacion_C|GetEST_Civi ets_civ))) 0 0)))
  (Variables|/Game/Blueprints/Mundo/BP_Civilizacion.BP_Civilizacion_C|SetEST_Civi ets_civ _output_get))

(fn GetESTEnumCivilizacion
  (params (bp_civilizacion :type BP%20Civilizacion%20Object%20Reference))
  (return (.civilizacion (Variables|/Game/Blueprints/Mundo/BP_Civilizacion.BP_Civilizacion_C|GetEST_Civi bp_civilizacion))))

(fn SetESTIntPoblacion
  (params (bp_civilizacion :type BP%20Civilizacion%20Object%20Reference) (poblacion :type Integer))
  (bind _est_civi (Variables|/Game/Blueprints/Mundo/BP_Civilizacion.BP_Civilizacion_C|GetEST_Civi bp_civilizacion))
  (bind _output_get (LocalVariables|Setest_civModificada (Utilities|Struct|MakeEST_Civilizacion (.civilizacion _est_civi) poblacion (.limitepoblacion _est_civi) (.comida _est_civi) (.npcs _est_civi) (.edificios _est_civi) 0 0)))
  (return _output_get))

(fn GetESTIntPoblacion
  (params (bp_civilizacion :type BP%20Civilizacion%20Object%20Reference))
  (return (.poblacion (Variables|/Game/Blueprints/Mundo/BP_Civilizacion.BP_Civilizacion_C|GetEST_Civi bp_civilizacion))))

(fn GetESTIntLimitePoblacion
  (params (bp_civilizacion :type BP%20Civilizacion%20Object%20Reference))
  (return (.limitepoblacion (Variables|/Game/Blueprints/Mundo/BP_Civilizacion.BP_Civilizacion_C|GetEST_Civi bp_civilizacion))))

(fn SetESTIntLimitePoblacion
  (params (bp_civilizacion :type BP%20Civilizacion%20Object%20Reference) (limitePoblacion :type Integer))
  (bind _est_civi (Variables|/Game/Blueprints/Mundo/BP_Civilizacion.BP_Civilizacion_C|GetEST_Civi bp_civilizacion))
  (bind _output_get (LocalVariables|Setest_civModificada (Utilities|Struct|MakeEST_Civilizacion (.civilizacion _est_civi) (.poblacion _est_civi) limitePoblacion (.comida _est_civi) (.npcs _est_civi) (.edificios _est_civi) 0 0)))
  (return _output_get))

(fn GetESTIntComida
  (params (bp_civilizacion :type BP%20Civilizacion%20Object%20Reference))
  (return (.comida (Variables|/Game/Blueprints/Mundo/BP_Civilizacion.BP_Civilizacion_C|GetEST_Civi bp_civilizacion))))

(fn SetESTIntComida
  (params (bp_civilizacion :type BP%20Civilizacion%20Object%20Reference) (comida :type Integer))
  (bind _est_civi (Variables|/Game/Blueprints/Mundo/BP_Civilizacion.BP_Civilizacion_C|GetEST_Civi bp_civilizacion))
  (bind _output_get (LocalVariables|Setest_civModificada (Utilities|Struct|MakeEST_Civilizacion (.civilizacion _est_civi) (.poblacion _est_civi) (.limitepoblacion _est_civi) comida (.npcs _est_civi) (.edificios _est_civi) 0 0)))
  (return _output_get))

(fn GetESTNpcsCivilizacion
  (params (bp_civilizacion :type BP%20Civilizacion%20Object%20Reference))
  (return (.npcs (Variables|/Game/Blueprints/Mundo/BP_Civilizacion.BP_Civilizacion_C|GetEST_Civi bp_civilizacion))))

(fn GetESTEdificiosCivilizacion
  (params (bp_civilizacion :type BP%20Civilizacion%20Object%20Reference))
  (return (.edificios (Variables|/Game/Blueprints/Mundo/BP_Civilizacion.BP_Civilizacion_C|GetEST_Civi bp_civilizacion))))

(fn SetESTNpcsCivilizacion
  (params (bp_civilizacion :type BP%20Civilizacion%20Object%20Reference) (Npcs :type Array%20of%20Actor%20Object%20References))
  (bind _est_civi (Variables|/Game/Blueprints/Mundo/BP_Civilizacion.BP_Civilizacion_C|GetEST_Civi bp_civilizacion))
  (bind _output_get (LocalVariables|Setest_civModificada (Utilities|Struct|MakeEST_Civilizacion (.civilizacion _est_civi) (.poblacion _est_civi) (.limitepoblacion _est_civi) (.comida _est_civi) Npcs (.edificios _est_civi) 0 0)))
  (return _output_get))

(fn SetESTEdificiosCivilizacion
  (params (bp_civilizacion :type BP%20Civilizacion%20Object%20Reference) (Edificios :type Array%20of%20Actor%20Object%20References))
  (bind _est_civi (Variables|/Game/Blueprints/Mundo/BP_Civilizacion.BP_Civilizacion_C|GetEST_Civi bp_civilizacion))
  (bind _output_get (LocalVariables|Setest_civModificada (Utilities|Struct|MakeEST_Civilizacion (.civilizacion _est_civi) (.poblacion _est_civi) (.limitepoblacion _est_civi) (.comida _est_civi) (.npcs _est_civi) Edificios 0 0)))
  (return _output_get))