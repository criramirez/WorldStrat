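; PlayerControllerCR is a player controller with keyboard shortcuts for testing and persisting the game's Reglas data.
; It caches GameInstanceCR in the construction script and uses it as the live store for Reglas.
; G sets a fixed Reglas value and opens NewMap, while H prints its Madeta field.
; O saves Reglas to a single SaveGameCR slot, creating it if missing, and L loads it back into the game instance.
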(event Input|KeyboardEvents|G
  (params (Key :type Key%20Structure))
  (:Pressed
    (Variables|/Game/Blueprints/BpGeneral/GameInstanceCR.GameInstanceCR_C|SetReglas (Variables|Default|GetGameInstance) (Utilities|Struct|MakeEST_Reglas 100))
    (Game|OpenLevel(byName) "NewMap")))

(event Input|KeyboardEvents|H
  (params (Key :type Key%20Structure))
  (:Pressed
    (Development|PrintString (Utilities|String|ToString(Integer) (.madeta (Variables|/Game/Blueprints/BpGeneral/GameInstanceCR.GameInstanceCR_C|GetReglas (Variables|Default|GetGameInstance)))))))

(event Input|KeyboardEvents|O
  (params (Key :type Key%20Structure))
  (:Pressed
    (bind _returnvalue (SaveGame|DoesSaveGameExist "SlotName"))
    (if _returnvalue
      (bind _returnvalue_2 (SaveGame|LoadGamefromSlot "SlotName"))
      (bind _assave_game_cr (Utilities|Casting|CastToSaveGameCR _returnvalue_2))
      (bind _output_get (Variables|Default|SetSaveSubClass _assave_game_cr))
      (Variables|/Game/Blueprints/BpGeneral/SaveGameCR.SaveGameCR_C|SetReglas _output_get (Variables|/Game/Blueprints/BpGeneral/GameInstanceCR.GameInstanceCR_C|GetReglas (Variables|Default|GetGameInstance)))
      (SaveGame|SaveGametoSlot (Variables|Default|GetSaveSubClass) "SlotName")
      (else
        (bind _returnvalue_3 (SaveGame|CreateSaveGameObject "/Game/Blueprints/BpGeneral/SaveGameCR.SaveGameCR_C"))
        (bind _output_get_2 (Variables|Default|SetSaveSubClass _returnvalue_3))
        (Variables|/Game/Blueprints/BpGeneral/SaveGameCR.SaveGameCR_C|SetReglas _output_get_2 (Variables|/Game/Blueprints/BpGeneral/GameInstanceCR.GameInstanceCR_C|GetReglas (Variables|Default|GetGameInstance)))
        (SaveGame|SaveGametoSlot (Variables|Default|GetSaveSubClass) "SlotName")))))

(event Input|KeyboardEvents|L
  (params (Key :type Key%20Structure))
  (:Pressed
    (bind _returnvalue (SaveGame|DoesSaveGameExist "SlotName"))
    (if _returnvalue
      (bind _returnvalue_2 (SaveGame|LoadGamefromSlot "SlotName"))
      (bind _assave_game_cr (Utilities|Casting|CastToSaveGameCR _returnvalue_2))
      (Variables|/Game/Blueprints/BpGeneral/GameInstanceCR.GameInstanceCR_C|SetReglas (Variables|Default|GetGameInstance) (Variables|/Game/Blueprints/BpGeneral/SaveGameCR.SaveGameCR_C|GetReglas _assave_game_cr)))))

(event Input|MouseEvents|LeftMouseButton
  (params (Key :type Key%20Structure)))

(event Input|TouchEvents|InputTouch
  (params (Location :type Vector) (FingerIndex :type ETouchIndex%20Enum)))

(fn ConstructionScript
  (bind _asgame_instance_cr (Utilities|Casting|CastToGameInstanceCR (Game|GetGameInstance)))
  (Variables|Default|SetGameInstance _asgame_instance_cr))