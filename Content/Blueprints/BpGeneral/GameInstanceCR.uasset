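; Game instance that holds the game's civilization data as structs, alongside their BP_Civilizacion actors.
; On Init it seeds two civilizations with a population limit and empty NPC and building lists.
; SetBpCivilizaciones spawns actors from the structs, and SetEstCiviliaciones copies actor state back into the struct array.
; Lookups return an actor by index or by civilization enum, the latter also re-setting the enum on the match.
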(event EventInit
  (CallFunction|Inicializar))

(fn SetEstCiviliaciones
  (Utilities|Array|Clear (Variables|Default|GetEST_Civ))
  (for _array_element (Variables|Default|GetBP_Civilizacion)
    (Utilities|Array|Add (Variables|Default|GetEST_Civ) (Variables|/Game/Blueprints/Mundo/BP_Civilizacion.BP_Civilizacion_C|GetEST_Civi _array_element))))

(fn SetBpCivilizaciones
  (Utilities|Array|Clear (Variables|Default|GetBP_Civilizacion))
  (for _array_element (Variables|Default|GetEST_Civ)
    (bind _returnvalue (Game|SpawnActorfromClass "/Game/Blueprints/Mundo/BP_Civilizacion.BP_Civilizacion_C" (Math|Transform|MakeTransform "0, 0, 0" "0, 0, 0" "1,1,1") "Undefined" 0 _array_element 0))
    (Utilities|Array|Add (Variables|Default|GetBP_Civilizacion) _returnvalue))
  (return (Variables|Default|GetBP_Civilizacion)))

(fn Inicializar
  (Variables|Default|SetEST_Civ (Utilities|Array|MakeArray (Utilities|Struct|MakeEST_Civilizacion "NewEnumerator0" 0 (Variables|Default|GetlimitePoblacionEst) 10 (Utilities|Array|MakeArray) (Utilities|Array|MakeArray)) (Utilities|Struct|MakeEST_Civilizacion "NewEnumerator1" 0 (Variables|Default|GetlimitePoblacionEst) 0 (Utilities|Array|MakeArray) (Utilities|Array|MakeArray)))))

(fn GetCivilizacion
  (params (PosArray :type Integer))
  (return (Utilities|Array|Get(acopy) (Variables|Default|GetBP_Civilizacion) PosArray)))

(fn BuscarCivilizacion
  (params (ENUM%20Civilizacion :type ENUM_Civilizaviones%20Enum :default "NewEnumerator2"))
  (for _array_element (Variables|Default|GetBP_Civilizacion)
    (bind _civilizacion (CallFunction|GetESTEnumCivilizacion _array_element))
    (if (Utilities|Enum|Equal(Enum) _civilizacion ENUM%20Civilizacion)
      (CallFunction|SetESTEnumCivilizacion ENUM%20Civilizacion _array_element)
      (return _array_element))))